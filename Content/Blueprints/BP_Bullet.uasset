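; BP_Bullet is a projectile actor used by both invaders and human shooters.
; On BeginPlay, the Invader flag selects an alien or human material and sets the ProjectileMovement speed, with human bullets flying faster.
; On overlap with any actor other than its Shooter, it sends DestroyMessage to that actor and destroys itself.
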(event OnComponentBeginOverlap(Bullet)
  (params (OverlappedComponent :type Primitive%20Component%20Object%20Reference) (OtherActor :type Actor%20Object%20Reference) (OtherComp :type Primitive%20Component%20Object%20Reference) (OtherBodyIndex :type Integer) (bFromSweep :type Boolean) (SweepResult :type Hit%20Result%20Structure%20%28by%20ref%29))
  ;[1 1 1] Destruction Logic
  (if (!= OtherActor (Variables|Default|GetShooter))
    (Class|BPIDestroy|Destroy(Message) OtherActor)
    (Actor|DestroyActor)))

(event EventBeginPlay
  (bind _bullet (Variables|Default|GetBullet))
  ;[1 1 1] Initialize Speed and Material
  (if (Variables|Default|GetInvader?)
    (Rendering|Material|SetMaterial _bullet 0 "/Game/Materials/M_AlienBullet.M_AlienBullet")
    (Variables|/Script/Engine.ProjectileMovementComponent|SetInitialSpeed (Variables|Default|GetProjectileMovement) 7e+02)
    (Variables|/Script/Engine.ProjectileMovementComponent|SetMaxSpeed (Variables|Default|GetProjectileMovement) 7e+02)
    (else
      (Rendering|Material|SetMaterial _bullet 0 "/Game/Materials/M_HumanBullet.M_HumanBullet")
      (Variables|/Script/Engine.ProjectileMovementComponent|SetInitialSpeed (Variables|Default|GetProjectileMovement) 9e+02)
      (Variables|/Script/Engine.ProjectileMovementComponent|SetMaxSpeed (Variables|Default|GetProjectileMovement) 9e+02))))

(fn ConstructionScript)