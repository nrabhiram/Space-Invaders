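; BP_Alien is a single Space Invaders-style enemy that marches, shoots and reports to its Army spawner.
; A self-repeating one-second Move loop steps it sideways, dropping and reversing at each edge, with a shorter first pass.
; It binds to the Army's shooter-selection event and fires a downward BP_Bullet when its ID is chosen.
; Each step sends the Army an invasion check against player height, and Destroy reports the kill.
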(event Custom|Move
  (bind _returnvalue (Transformation|GetActorLocation))
  (bind _returnvalue_2 (Transformation|GetActorLocation))
  ;[1 1 1] Marching Logic
  (Utilities|FlowControl|Sequence
    (:then_0
      (if (Variables|Default|GetFirst%20March)
        (Variables|Default|SetMaximum%20Move%20Length 8)
        (else
          (Variables|Default|SetMaximum%20Move%20Length 16)))
      (if (== (Variables|Default|GetMove%20Id) (Variables|Default|GetMaximum%20Move%20Length))
        (Utilities|FlowControl|Sequence
          (:then_0
            (Transformation|SetActorLocation (Math|Vector|MakeVector (.x _returnvalue) (.y _returnvalue) (- (.z _returnvalue) 1.2e+02)) false false)
            (Variables|Default|SetMove%20Id 0)
            (if (== (Variables|Default|GetDirection) 1)
              (Variables|Default|SetDirection -1)
              (else
                (Variables|Default|SetDirection 1))))
          (:then_1
            (if (Variables|Default|GetFirst%20March)
              (Variables|Default|SetFirst%20March false))))
        (else
          (Transformation|SetActorLocation (Math|Vector|MakeVector (.x _returnvalue_2) (+ (.y _returnvalue_2) (* (Variables|Default|GetDirection) 2e+01)) (.z _returnvalue_2)) false false)
          (Variables|Default|SetMove%20Id (+ (Variables|Default|GetMove%20Id) 1)))))
    (:then_1
      (CallFunction|CheckifSuccesfullyInvaded)
      (Utilities|FlowControl|Delay 1.0)
      (CallFunction|Move))))

(event Custom|On%20Alien%20Shooter%20Selected
  (params (Selected%20Shooter :type S%20Alien%20Structure))
  (bind (_id _alive_) (Utilities|Struct|BreakS_Alien Selected%20Shooter))
  (bind _defaultsceneroot (Variables|Default|GetDefaultSceneRoot))
  (bind _returnvalue (Transformation|GetWorldTransform _defaultsceneroot))
  ;[1 1 1] Shooter Selected Bind Event - check if selected shooter is equal to alien and spawn bullet accordingly
  (if (and (== _id (Utilities|Struct|BreakS_Alien (Variables|Default|GetAlien%20Data))) _alive_)
    (Game|SpawnActorfromClass "/Game/Blueprints/BP_Bullet.BP_Bullet_C" (Math|Transform|MakeTransform (.location _returnvalue) (Math|Rotator|MakeRotator (.roll (.rotation _returnvalue)) -9e+01 (.yaw (.rotation _returnvalue))) (.scale _returnvalue)) "Undefined" 0 self true 0)))

(event Custom|Check%20if%20Succesfully%20Invaded
  (Default|OnSuccesfulInvasion (Variables|Default|GetArmy) (<= (.z (Transformation|GetActorLocation)) (.z (Transformation|GetActorLocation (Game|GetPlayerCharacter 0))))))

(event EventBeginPlay
  ;[1 1 1] Initialize alien by binding event to "Shooter Selected" in spawner blueprint and beginning the marching tick
  (bind _army (Variables|Default|GetArmy)
    (:then
      (EventDispatchers|BindEventtoAlienShooterSelected _army (EventDispatchers|CreateEvent :!event Custom|On%20Alien%20Shooter%20Selected))
      (CallFunction|Move))
    (:else)))

(event EventDestroy
  ;[1 1 1] Destroy Event - called when bullet touches alien
  (Default|OnAlienKilled (Variables|Default|GetArmy) (Utilities|Struct|BreakS_Alien (Variables|Default|GetAlien%20Data)))
  (Actor|DestroyActor))

(fn ConstructionScript)