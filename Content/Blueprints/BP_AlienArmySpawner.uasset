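; Spawns and controls a Space Invaders-style alien army as a grid above the player, with mesh and points set by row.
; A one-second recursive tick broadcasts sideways marches, or a forward march and direction flip when a living alien reaches a boundary.
; Sideways ticks also pick a random shooter from aliens with no living column-mate below.
; Tracks alien deaths and positions, calling Win when all die and Lose on successful invasion.
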(event Custom|Alien%20Marching%20Tick
  ;[1 1 1] Determine who is supposed to shoot at the next tick
  (Utilities|FlowControl|Sequence
    (:then_0
      (if (and (Utils|DidAlienReachBoundary) (!= (Variables|MarchingLogic|GetTicks%20Since%20Forward%20March) 1))
        (Default|CallMarchForward)
        (Variables|MarchingLogic|SetTicks%20Since%20Forward%20March 0)
        (if (== (Variables|MarchingLogic|GetDirection) 1)
          (Variables|MarchingLogic|SetDirection -1)
          (else
            (Variables|MarchingLogic|SetDirection 1)))
        (else
          (bind _selected_shooter (DetermineShooter|SelectAlienShooter))
          (Default|CallAlienShooterSelected _selected_shooter)
          (Default|CallAlienMarch (Variables|MarchingLogic|GetDirection)))))
    (:then_1
      (Math|Integer|IncrementInt (Variables|MarchingLogic|GetTicks%20Since%20Forward%20March)
        (:%20%20
          (Utilities|FlowControl|Delay 1.0)
          (CallFunction|AlienMarchingTick))))))

(event Custom|On%20Succesful%20Invasion
  (params (Success :type Boolean))
  ;[1 1 1] If army successfully invades player, player loses the game
  (if Success
    (bind _asside_scroller_character (Utilities|Casting|CastToSideScrollerCharacter (Game|GetPlayerCharacter 0)))
    (Default|Lose _asside_scroller_character)))

(event Custom|Update%20Alien%20Location
  (params (Index :type Integer) (Updated%20Location :type Vector))
  ;[1 1 1] Update Alien Location
  (Utilities|Array|SetArrayElem (Variables|AlienArmyData|GetAlien%20Locations) Index Updated%20Location))

(event EventBeginPlay
  ;[1 1 1] Initialize army grid
  (for _index (range 0 (- (* (Variables|Grid|GetRows) (Variables|Grid|GetColumns)) 1))
    (Initialization|AddAlientoList _index)
    (Initialization|SpawnAlien _index))
  (CallFunction|AlienMarchingTick))

(fn ConstructionScript)

(fn LocateAlienPosition
  (params (Index :type Integer))
  (bind _columns (Variables|Grid|GetColumns))
  (bind _returnvalue (Math|Conversions|ToFloat(Integer) Index))
  (bind _returnvalue_2 (Math|Conversions|ToFloat(Integer) _columns))
  (bind (_remainder _returnvalue_3) (Math|Float|Division(WholeandRemainder) _returnvalue _returnvalue_2))
  (return _returnvalue_3 (Math|Float|Truncate _remainder)))

(fn AddAlientoList
  (params (Index :type Integer))
  (bind (_row _column) (Utils|LocateAlienPosition Index))
  (Utilities|Array|Add (Variables|AlienArmyData|GetAlien%20Army) (Utilities|Struct|MakeS_Alien Index _row _column true)))

(fn SpawnAlien
  (params (Index :type Integer))
  (bind (_row _column) (Utils|LocateAlienPosition Index))
  (bind _returnvalue (Game|Player|GetPlayerPawn 0))
  (bind _grid_distance (Variables|Grid|GetGrid%20Distance))
  (bind _columns (Variables|Grid|GetColumns))
  (bind _actor_spacing (Variables|Grid|GetActor%20Spacing))
  (bind _actor_spacing_2 (Variables|Grid|GetActor%20Spacing))
  (bind _returnvalue_2 (Transformation|GetActorLocation _returnvalue))
  (bind _returnvalue_3 (* _row _actor_spacing))
  (bind _returnvalue_4 (/ _columns 2))
  (bind _returnvalue_5 (- _column _returnvalue_4))
  (bind _returnvalue_6 (+ (.z _returnvalue_2) _grid_distance))
  (bind _returnvalue_7 (* _returnvalue_5 _actor_spacing_2))
  (bind _returnvalue_8 (+ _returnvalue_3 _returnvalue_6))
  (bind _returnvalue_9 (+ _returnvalue_7 (.y _returnvalue_2)))
  (Game|SpawnActorfromClass "/Game/Blueprints/BP_Alien.BP_Alien_C" (Math|Transform|MakeTransform (Math|Vector|MakeVector (.x _returnvalue_2) _returnvalue_9 _returnvalue_8) "0, 0, 0" "1,1,1") "Undefined" 0 self (Utilities|Array|Get(acopy) (Variables|AlienArmyData|GetAlien%20Army) Index) (Utils|CalculateAlienPoints _row) (Utils|CalculateMarchingDistance) (Utils|CalculateAlienMesh _row) 0)
  (Utilities|Array|Add (Variables|AlienArmyData|GetAlien%20Locations) (Math|Vector|MakeVector (.x _returnvalue_2) _returnvalue_9 _returnvalue_8)))

(fn SelectAlienShooter
  ;[1 1 1] Find potential shooters
  (for (_array_element _array_index) (Variables|AlienArmyData|GetAlien%20Army)
    (if (Utils|IsShotPathClear _array_index)
      (Utilities|Array|Add (LocalVariables|GetL%20Aliens%20that%20Can%20Shoot) _array_element)))
  ;[1 1 1] Randomly determine the shooter
  (bind (_array_element_2 _array_index_2) (Utilities|Array|ForEachLoopwithBreak (LocalVariables|GetL%20Aliens%20that%20Can%20Shoot) :!label _label)
    (:LoopBody
      (LocalVariables|SetL%20Selected%20Shooter _array_element_2)
      (if (Math|Random|RandomBoolwithWeight (* (+ _array_index_2 1) (/ 1.0 (Math|Conversions|ToFloat(Integer) (- (Utilities|Array|Length (LocalVariables|GetL%20Aliens%20that%20Can%20Shoot)) 1)))))
        (goto _label Break)))
    (:Completed
      (return (LocalVariables|GetL%20Selected%20Shooter)))))

(fn IsShotPathClear
  (params (Index :type Integer))
  (return (and (Utils|IsAlienAlive Index) (== (Utilities|Array|Length (Utils|GetColumnMates Index)) 0))))

(fn OnAlienKilled
  (params (Index :type Integer))
  (bind _alien_army (Variables|AlienArmyData|GetAlien%20Army))
  (bind _output (Utilities|Array|Get(acopy) _alien_army Index))
  (bind (_id _row _column) (Utilities|Struct|BreakS_Alien _output))
  (Utilities|Array|SetArrayElem (Variables|AlienArmyData|GetAlien%20Army) Index (Utilities|Struct|MakeS_Alien _id _row _column false))
  (Math|Integer|IncrementInt (Variables|AlienArmyData|GetNum%20Dead)
    (:%20%20
      (if (== (Variables|AlienArmyData|GetNum%20Dead) (Utilities|Array|Length (Variables|AlienArmyData|GetAlien%20Army)))
        (bind _asside_scroller_character (Utilities|Casting|CastToSideScrollerCharacter (Game|GetPlayerCharacter 0)))
        (Default|Win _asside_scroller_character)))))

(fn IsAlienAlive
  (params (Index :type Integer))
  (return (Utilities|Struct|BreakS_Alien (Utilities|Array|Get(acopy) (Variables|AlienArmyData|GetAlien%20Army) Index))))

(fn GetColumnMates
  (params (Index :type Integer))
  (bind _alien_army (Variables|AlienArmyData|GetAlien%20Army))
  (bind _output (Utilities|Array|Get(acopy) _alien_army Index))
  (bind (_id _row _column) (Utilities|Struct|BreakS_Alien _output))
  (for _array_element (Variables|AlienArmyData|GetAlien%20Army)
    (if (Math|Boolean|ANDBoolean (!= (.ID (Utilities|Struct|BreakS_Alien _array_element)) _id) (== (.Column (Utilities|Struct|BreakS_Alien _array_element)) _column) (> _row (.Row (Utilities|Struct|BreakS_Alien _array_element))) (.Alive? (Utilities|Struct|BreakS_Alien _array_element)))
      (Utilities|Array|Add (LocalVariables|GetL%20Column%20Mates) _array_element)))
  (return (LocalVariables|GetL%20Column%20Mates)))

(fn CalculateAlienPoints
  (params (Row%20Index :type Integer))
  (if (Math|Integer|InRange(Integer) Row%20Index 0 1)
    (return 1e+01)
    (elif (Math|Integer|InRange(Integer) Row%20Index 2 3)
      (return 2e+01)
      (else
        (return 3e+01)))))

(fn DidAlienReachBoundary
  (bind (_array_element _array_index) (Utilities|Array|ForEachLoopwithBreak (Variables|AlienArmyData|GetAlien%20Army) :!label _label)
    (:LoopBody
      (if (.Alive? (Utilities|Struct|BreakS_Alien _array_element))
        (bind _output_get (LocalVariables|SetL%20Boundary%20Reached (or (>= (.y (Utilities|Array|Get(acopy) (Variables|AlienArmyData|GetAlien%20Locations) _array_index)) (.y (Variables|MarchingLogic|GetUpper%20Bound))) (<= (.y (Utilities|Array|Get(acopy) (Variables|AlienArmyData|GetAlien%20Locations) _array_index)) (.y (Variables|MarchingLogic|GetLower%20Bound))))))
        (if _output_get
          (goto _label Break))))
    (:Completed
      (return (LocalVariables|GetL%20Boundary%20Reached)))))

(fn CalculateMarchingDistance
  (return (/ (* 2 (Variables|Grid|GetActor%20Spacing)) 8.0)))

(fn CalculateAlienMesh
  (params (Row%20Index :type Integer))
  (if (Math|Integer|InRange(Integer) Row%20Index 0 1)
    (return "/Game/Models/Alien_1.Alien_1")
    (elif (Math|Integer|InRange(Integer) Row%20Index 2 3)
      (return "/Game/Models/Alien_2.Alien_2")
      (else
        (return "/Game/Models/Alien_3.Alien_3")))))