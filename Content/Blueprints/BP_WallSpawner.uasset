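; BP_WallSpawner builds several brick walls above the player pawn at BeginPlay, apparently as shields in an alien-invasion shooter.
; Each wall is a grid of BP_Brick actors, with a flat index converted to row and column by division and remainder.
; Bricks share the pawn's X, rows stack upward in Z, and columns spread along Y using alien army width, wall gap and hardcoded offsets.
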(event EventBeginPlay
  ;[1 1 1] Initialize Walls
  (for _index (range 0 (- (Variables|Default|GetNum%20Walls) 1))
    (for _index_2 (range 0 (- (* (Variables|Default|GetRows) (Variables|Default|GetColumns)) 1))
      (Game|SpawnActorfromClass "/Game/Blueprints/BP_Brick.BP_Brick_C" (Math|Transform|MakeTransform (Math|Vector|MakeVector (.x (Transformation|GetActorLocation (Game|Player|GetPlayerPawn 0))) (Utils|GetColumnLocation (.Column (Utils|LocateBrickPosition _index_2)) _index) (Utils|GetRowLocation (.Row (Utils|LocateBrickPosition _index_2)))) "0, 0, 0" "1,1,1") "Undefined" 0 0))))

(fn ConstructionScript)

(fn LocateBrickPosition
  (params (Index :type Integer))
  (bind _returnvalue (Math|Conversions|ToFloat(Integer) Index))
  (bind _columns (Variables|Default|GetColumns))
  (bind _returnvalue_2 (Math|Conversions|ToFloat(Integer) _columns))
  (bind (_remainder _returnvalue_3) (Math|Float|Division(WholeandRemainder) _returnvalue _returnvalue_2))
  (return _returnvalue_3 (Math|Float|Truncate _remainder)))

(fn GetRowLocation
  (params (Row%20Index :type Integer))
  (return (+ (* Row%20Index (Variables|Default|GetActor%20Spacing)) (+ (.z (Transformation|GetActorLocation (Game|Player|GetPlayerPawn 0))) (Variables|Default|GetGrid%20Distance)))))

(fn GetColumnLocation
  (params (Column%20Index :type Integer) (Wall%20Index :type Integer))
  (return (+ (* (- Column%20Index 2) (Variables|Default|GetActor%20Spacing)) (- (+ (.y (Transformation|GetActorLocation (Game|Player|GetPlayerPawn 0))) (* (Math|Conversions|ToFloat(Integer) (/ (Variables|Default|GetArmy%20Columns) 2)) (Variables|Default|GetAlien%20Size))) (+ 52.5 (* Wall%20Index (+ (* (Variables|Default|GetNum%20Walls) (Variables|Default|GetActor%20Spacing)) (Variables|Default|GetWall%20Gap%20Spacing))))))))